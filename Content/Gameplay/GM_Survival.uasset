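; Survival game mode that runs pooled enemy waves and returns to the main menu on victory or player defeat.
; State changes toggle pause, and entering Playing from MainMenu fills the SpawnManager's pool and spawns enemies.
; Defeated enemies are reported to GameStateSurvival, then a random inactive one respawns at a random CharacterSpawner after a delay.
; GameStateSurvival drives the score widget and signals victory, while the player's CombatComponent signals defeat.
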(event `EventOnStateChanged`
  (params (PreviousState :type "/Game/Gameplay/E_GameState Enum" :default "NewEnumerator0") (NewState :type "/Game/Gameplay/E_GameState Enum" :default "NewEnumerator0"))
  (switch `/Game/Gameplay/E_GameState` NewState
    (:`NewEnumerator1`
      ;[1 1 1] Pause the game
      (if (not (`GameplayStatics.IsGamePaused`))
        (`GameplayStatics.SetGamePaused` true)))
    (:`NewEnumerator2`
      (`|ExecutionSequence`
        (:`then_0`
          ;[1 1 1] Unpuse the game if needed
          (if (and (`|EnumEquality` PreviousState "NewEnumerator1") (`GameplayStatics.IsGamePaused`))
            (`GameplayStatics.SetGamePaused` false)))
        (:`then_1`
          (if (`|EnumEquality` PreviousState "NewEnumerator0")
            (`self.EventSpawnEnemies`)))))))

(event `self.ReceiveBeginPlay`
  (`|ExecutionSequence`
    (:`then_1`
      ;[1 1 1] Adding UI to viewport
      (bind _returnvalue (`|CreateWidget` "/Game/UI/WB_GameUI.WB_GameUI_C"))
      (set `self.T Score` (`/Game/UI/WB_GameUI.tScore` _returnvalue))
      (`UserWidget.AddToViewport` _returnvalue 0)
      (`TextBlock.SetText` (`self.T Score`) (`KismetTextLibrary.Conv_StringToText` (`GameStateSurvival.GetFormattedScore` (`self.CurrentGameState`)))))
    (:`then_2`
      ;[1 1 1] Bind Score changed event
      (add `GameStateSurvival.OnScoreChanged` (`self.CurrentGameState`) (`|CreateDelegate` :!event `EventOnScoreChanged`)))
    (:`then_4`
      ;[1 1 1] Setup SpawnManager and EnemySpawners
      (bind _asgame_state_survival (cast `GameStateSurvival` (`GameplayStatics.GetGameState`)))
      (bind _output_get (set `self.CurrentGameState` _asgame_state_survival))
      (add `GameStateSurvival.OnAllEnemiesDefeated` _output_get (delegate `OnAllEnemiesDefeated`))
      (set `GameStateSurvival.DefeatedEnemyCountToWin` (`self.Defeated Enemy Count To Win`) _output_get))
    (:`then_5`)))

(event `EventSpawnEnemies`
  ;[1 1 1] Initialize enemies TODO: use SpawnManager for these operations
  (bind _returnvalue (`SpawnManager.InitEnemyPool` (`self.SpawnManager`) (`|MakeArray` (make `SpawnParams` "/Game/Characters/AI/BP_BasicEnemy.BP_BasicEnemy_C" "/Game/Characters/AI/BT_BasicEnemy.BT_BasicEnemy" (`self.PooledEnemyCount`)))))
  (`KismetSystemLibrary.LogString` (`KismetStringLibrary.BuildString_Int` "Initializing " "" (`KismetArrayLibrary.Array_Length` _returnvalue) " enemies"))
  (for _array_element _returnvalue
    (if (`KismetSystemLibrary.DoesImplementInterface` _array_element "/Script/TopDown2.EnemyCharacterInterface")
      (message `EnemyCharacterInterface.BindOnDefeatedEvent` _array_element self)
      (`KismetSystemLibrary.Delay` 1.0)
      (`SpawnManager.SpawnEnemiesOnAllSpawnersFromPoolTop` (`self.SpawnManager`))
      (`KismetSystemLibrary.PrintString` "Hello")
      (else
        (`KismetSystemLibrary.PrintString` "Invalid enemy interface")))))

(event `OnAllEnemiesDefeated`
  ;[1 1 1] Handle game clear
  (`GameplayStatics.PlaySoundAtLocation` "/Game/Audio/Explosion02.Explosion02" (0.0 0.0 0.0) (struct) 1.0 1.0 0.0 null null null null)
  (`KismetSystemLibrary.Delay` 3.0)
  (`GameplayStatics.OpenLevelBySoftObjectPtr` "/Game/LevelPrototyping/Maps/L_MainMenu.L_MainMenu"))

(event `OnPlayerDefeated`
  (params (Owner :type "Object Object Reference"))
  ;[1 1 1] Player defeat
  (`KismetSystemLibrary.LogString` "Player defeated! AAAA")
  (`KismetSystemLibrary.Delay` 3.0)
  (`GameplayStatics.OpenLevelBySoftObjectPtr` "/Game/LevelPrototyping/Maps/L_MainMenu.L_MainMenu"))

(event `OnPlayerSpawned_Event`
  (add `CombatComponent.OnDefeat` (`self.GetComponentByClass` (`GameplayStatics.GetPlayerPawn` 0) "/Script/TopDown2.CombatComponent") (delegate `OnPlayerDefeated`)))

(event `self.OnEnemyDefeated`
  (params (Enemy :type "Object Object Reference"))
  (bind _asenemy_character_interface (cast `EnemyCharacterInterface` Enemy)
    (:`then`
      (bind _returnvalue (`KismetSystemLibrary.Conv_InterfaceToObject` _asenemy_character_interface))
      ;[1 1 1] Reset defeated enemy
      (`/Game/Gameplay/BP_SpawnManager.OnEnemyDefeated_Event` (`.SpawnManager` (`self.SpawnManager`)) _returnvalue)
      (bind _returnvalue_2 (message `EnemyCharacterInterface.GetCharacter` _returnvalue))
      (`GameStateSurvival.HandleEnemyDefeated` (`self.CurrentGameState`) _returnvalue_2)
      (`KismetSystemLibrary.Delay` 5.0)
      (bind _returnvalue_3 (`SpawnManager.GetRandomInactiveEnemyFromPool` (`self.SpawnManager`)))
      (bind _returnvalue_4 (`KismetSystemLibrary.Conv_InterfaceToObject` _returnvalue_3))
      (`/Engine/EditorBlueprintResources/StandardMacros.IsValid` _returnvalue_4
        (:`Is Valid`
          (bind _outactors (`GameplayStatics.GetAllActorsOfClass` "/Script/TopDown2.CharacterSpawner"))
          (`SpawnManager.SpawnEnemy` (`self.SpawnManager`) _returnvalue_4 (`KismetArrayLibrary.Array_Random` _outactors)))))
    (:`CastFailed`
      (`KismetSystemLibrary.LogString` "Invalid enemy class!")
      (`KismetSystemLibrary.QuitGame` null "Quit"))))

(event `EventOnScoreChanged`
  (params (GameMode :type "GameMode Object Reference") (NewValue :type Integer) (OldValue :type Integer))
  ;[1 1 1] Update score text
  (`TextBlock.SetText` (`self.T Score`) (`KismetTextLibrary.Conv_IntToText` NewValue)))

(fn `ChangeState`
  (params (NewState :type "/Game/Gameplay/E_GameState Enum" :default "NewEnumerator0") (PreviousState :type "/Game/Gameplay/E_GameState Enum" :default "NewEnumerator0"))
  (bind _output_get (set `self.CurrentState` NewState))
  (`self.EventOnStateChanged` PreviousState _output_get))

(fn `UserConstructionScript`)