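; Game mode Blueprint for the main menu, handling its camera, UI and start and quit actions.
; On BeginPlay it points the first player's view at a CameraActor found in the level and adds the WB_MainMenuUI widget to the viewport.
; It binds the widget's buttons from the game mode itself: Start opens TopDownMap and Quit exits the game.
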(event `self.ReceiveBeginPlay`
  (set `self.bFindCameraComponentWhenViewTarget` true)
  (bind _returnvalue (`GameplayStatics.GetActorOfClass` "/Script/Engine.CameraActor"))
  (`PlayerController.SetViewTargetWithBlend` (`GameplayStatics.GetPlayerController` 0) _returnvalue 0.0 "VTBlend_Linear" 0.0 false)
  (bind _returnvalue_2 (`|CreateWidget` "/Game/UI/WB_MainMenuUI.WB_MainMenuUI_C"))
  (`UserWidget.AddToViewport` _returnvalue_2 0)
  (add `Button.OnClicked` (`/Game/UI/WB_MainMenuUI.bStartGame` _returnvalue_2) (`|CreateDelegate` :!event `OnClickedStart`))
  (add `Button.OnClicked` (`/Game/UI/WB_MainMenuUI.bQuitGame` _returnvalue_2) (`|CreateDelegate` :!event `OnClickedQuit`)))

(event `OnClickedStart`
  (`GameplayStatics.OpenLevelBySoftObjectPtr` "/Game/LevelPrototyping/Maps/TopDownMap.TopDownMap"))

(event `OnClickedQuit`
  (`KismetSystemLibrary.QuitGame` null "Quit"))

(fn `UserConstructionScript`)