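; Survival game mode that tracks score and remaining enemies, showing score in a debug UI.
; On BeginPlay it has BP_SpawnManager load and position enemies, and binds score changes and the character's score-add input.
; Defeated enemies are recycled: hidden, forget the player, move to a random spawner, regain health and reappear after a delay.
; Each defeat adds score and lowers the remaining count, calling a still-empty game-clear function at zero.
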(event `self.ReceiveBeginPlay`
  (`|ExecutionSequence`
    (:`then_0`
      ;[1 1 1] Adding UI to viewport
      (bind _returnvalue (`|CreateWidget` "/Game/UI/BP_DebugUI.BP_DebugUI_C"))
      (set `self.T Score` (`/Game/UI/BP_DebugUI.tScore` _returnvalue))
      (`UserWidget.AddToViewport` _returnvalue 0)
      (`TextBlock.SetText` (`self.T Score`) (`KismetTextLibrary.Conv_StringToText` (`self.GetFormattedScore`))))
    (:`then_1`
      ;[1 1 1] Bind Score changed event
      (add `self.OnScoreChanged` (`|CreateDelegate` :!event `EventOnScoreChanged`)))
    (:`then_2`
      (bind _asbp_top_down_character (cast `/Game/Characters/Player/BP_TopDownCharacter` (`GameplayStatics.GetPlayerCharacter` 0)))
      (add `/Game/Characters/Player/BP_TopDownCharacter.OnScoreAddPressed` _asbp_top_down_character (delegate `EventScoreAddPressed`)))
    (:`then_3`
      (bind _returnvalue_2 (`GameplayStatics.GetActorOfClass` "/Game/Gameplay/BP_SpawnManager.BP_SpawnManager_C"))
      (set `self.SpawnManager` _returnvalue_2)
      (`self.EventSpawnEnemies`))))

(event `EventSpawnEnemies`
  (bind _asbp_spawn_manager (cast `/Game/Gameplay/BP_SpawnManager` (`self.SpawnManager`)))
  (`/Game/Gameplay/BP_SpawnManager.EventLoadEnemiesAtSpawns` _asbp_spawn_manager)
  (`/Game/Gameplay/BP_SpawnManager.EventMoveEnemiesToSpawns` _asbp_spawn_manager))

(event `EventOnScoreChanged` :!signature `self.OnScoreChanged`
  (params (GameMode :type "GameMode Object Reference") (NewValue :type Integer) (OldValue :type Integer))
  ;[1 1 1] Update score text
  (`TextBlock.SetText` (`self.T Score`) (`KismetTextLibrary.Conv_IntToText` NewValue)))

(event `EventScoreAddPressed`
  (bind _returnvalue (+ (`self.GetScore`) 100))
  (`self.SetScore` _returnvalue)
  (`self.EventOnScoreChanged` null _returnvalue (`self.GetScore`)))

(event `OnEnemyDefeated_Event`
  (params (HealthComponent :type "HealthComponent Object Reference") (Character :type "Character Object Reference") (AIController :type "AIController Object Reference"))
  (`|ExecutionSequence`
    (:`then_0`
      ;[1 1 1] Forget player's location/reference
      (`BlackboardComponent.SetValueAsObject` (`AIController.Blackboard` AIController) "KeyPlayerCharacter" null))
    (:`then_1`
      ;[1 1 1] Move defeated enenemy to random spawn
      (`self.SetActorHiddenInGame` Character true))
    (:`then_2`
      (`/Game/Gameplay/BP_SpawnManager.EventSpawnEnemyAtRandomSpawner` (`self.SpawnManager`) Character))
    (:`then_3`
      (`KismetSystemLibrary.Delay` 5.0)
      (`self.SetActorHiddenInGame` Character false))
    (:`then_4`
      (set `HealthComponent.CurrentHealth` (`HealthComponent.GetMaxHealth` HealthComponent) HealthComponent))
    (:`then_5`
      (`self.SetScore` (+ (`self.GetScore`) 100))
      (`TextBlock.SetText` (`self.T Score`) (`KismetTextLibrary.Conv_StringToText` (`self.GetFormattedScore`)))
      (bind _output_get (set `self.EnemiesLeftCount` (- (`self.EnemiesLeftCount`) 1)))
      (if (<= _output_get 0)
        (`self.PlayGameClearScenario`)))))

(fn `PlayGameClearScenario`)

(fn `UserConstructionScript`)