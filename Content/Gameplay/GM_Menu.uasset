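; Game mode for the main menu that shows the menu screen and handles starting or quitting the game.
; On BeginPlay it blends the first player's view to a CameraActor in the level, adds the WB_MainMenuScreen widget to the viewport and shows the mouse cursor.
; The widget's start and quit dispatchers are bound to events that open TopDownMap or quit the application.
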(event `self.ReceiveBeginPlay`
  (`|ExecutionSequence`
    (:`then_0`
      (set `self.bFindCameraComponentWhenViewTarget` true)
      (bind _returnvalue (`GameplayStatics.GetActorOfClass` "/Script/Engine.CameraActor"))
      (`PlayerController.SetViewTargetWithBlend` (`GameplayStatics.GetPlayerController` 0) _returnvalue 0.0 "VTBlend_Linear" 0.0 false))
    (:`then_1`
      (bind _returnvalue_2 (`|CreateWidget` "/Game/UI/Screens/WB_MainMenuScreen.WB_MainMenuScreen_C"))
      (bind _output_get (set `self.WB_MainMenu` _returnvalue_2))
      (`UserWidget.AddToViewport` _output_get 0)
      (add `/Game/UI/Screens/WB_MainMenuScreen.OnStartGameClicked` (`self.WB_MainMenu`) (`|CreateDelegate` :!event `EventStartGame`))
      (add `/Game/UI/Screens/WB_MainMenuScreen.OnQuitGameClicked` (`self.WB_MainMenu`) (`|CreateDelegate` :!event `EventQuitGame`)))
    (:`then_2`
      (bind _returnvalue_3 (`InputDeviceLibrary.GetPlayerControllerFromInputDevice` (struct)))
      (set `PlayerController.bShowMouseCursor` true _returnvalue_3))))

(event `EventStartGame`
  (`GameplayStatics.OpenLevelBySoftObjectPtr` "/Game/LevelPrototyping/Maps/TopDownMap.TopDownMap"))

(event `EventQuitGame`
  (`KismetSystemLibrary.QuitGame` null "Quit"))

(fn `UserConstructionScript`)