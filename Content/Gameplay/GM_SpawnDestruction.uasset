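; Game mode for the Spawn Destruction level, where the player fights pooled drones and destroys physical spawners.
; On BeginPlay it initializes the drone pool, registers spawners with GameStateSpawnDestruction and creates the game screen widget.
; It relays spawn and defeat events to the game state, whose change events update the HUD alongside player health.
; Level clear and player defeat both show the level-cleared text, then open the main menu after a delay.
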(event `self.K2_PostLogin`
  (params (NewPlayer :type "PlayerController Object Reference"))
  ;[1 1 1] Binding to player's spawn event. TODO: add this in base C++
  (add `Controller.OnPossessedPawnChanged` NewPlayer (`|CreateDelegate` :!event `EventOnPlayerSpawned`)))

(event `self.ReceiveBeginPlay`
  (`|ExecutionSequence`
    (:`then_0`
      ;[1 1 1] Setup level
      ;;[1 1 1] Init enemies and bind to their events
      (`self.InitEnemies` (`|MakeArray` (make `SpawnParams` "/Game/Characters/Drone/BP_Drone.BP_Drone_C" "/Game/Characters/Drone/BT_Drone.BT_Drone" (`self.PooledEnemyCount`))))
      (bind _returnvalue (`self.GetSpawnManager`))
      (bind _returnvalue_2 (`SpawnManager.GetInactiveEnemies` _returnvalue))
      (for _array_element _returnvalue_2
        (bind _returnvalue_3 (message `EnemyCharacterInterface.GetCombatComponent` _array_element))
        (add `CombatComponent.OnDefeatStarted` _returnvalue_3 (`|CreateDelegate` :!event `EventOnEnemyDefeatStarted`))))
    (:`then_1`
      ;;[1 1 1] Bind to level clear event, enemy and spawner count changed events
      (bind _asgame_state_spawn_destruction (cast `GameStateSpawnDestruction` (`GameplayStatics.GetGameState`)))
      (bind _output_get (set `self.CurrentGameState` _asgame_state_spawn_destruction))
      (add `GameStateSpawnDestruction.OnLevelCleared` _output_get (`|CreateDelegate` :!event `EventLevelCleared`))
      (add `GameStateSpawnDestruction.OnEnemyCountChanged` (`self.CurrentGameState`) (delegate `EventOnEnemyCountChanged`))
      (add `GameStateSpawnDestruction.OnSpawnerCountChanged` (`self.CurrentGameState`) (delegate `EventOnSpawnerCountChanged`))
      (add `GameStateSpawnDestruction.OnScoreChanged` (`self.CurrentGameState`) (delegate `EventOnScoreChanged`)))
    (:`then_2`
      (`|ExecutionSequence`
        (:`then_0`
          ;;[1 1 1] Bind on spawner events
          (bind _outactors (`GameplayStatics.GetAllActorsOfClass` "/Game/Characters/PhysicalSpawner/BP_PhysicalSpawner.BP_PhysicalSpawner_C"))
          ;;;[1 1 1] TODO: add Get in base class
          (`GameStateSpawnDestruction.SetSpawners` (`self.CurrentGameState`) _outactors)
          (bind _output_get_2 (set `self.Out Actors` _outactors))
          (for _array_element_2 _output_get_2
            (add `CombatComponent.OnDefeatStarted` (`self.GetComponentByClass` _array_element_2 "/Script/TopDown2.CombatComponent") (`|CreateDelegate` :!event `EventOnSpawnerDestroyed`))))
        (:`then_1`
          ;;;[1 1 1] TODO: probably spawners should fire these events
          (bind _returnvalue_4 (`self.GetSpawnManager`))
          (add `SpawnManager.OnEnemySpawned` _returnvalue_4 (`|CreateDelegate` :!event `OnEnemySpawned`)))))
    (:`then_3`
      ;[1 1 1] Adding UI to viewport
      (bind _returnvalue_5 (`|CreateWidget` "/Game/UI/Screens/WB_GameScreen.WB_GameScreen_C"))
      (bind _output_get_3 (set `self.GameScreenWidget` _returnvalue_5))
      (`UserWidget.AddToViewport` _output_get_3 0))
    (:`then_4`
      (`/Game/UI/Screens/WB_GameScreen.ShowGameStateText` (`self.GameScreenWidget`) (`self.LevelStartText`))
      (`KismetSystemLibrary.K2_SetTimerDelegate` (`|CreateDelegate` :!event `HideGameStateText`) (`self.LevelStartDisplayTime`)))))

(event `EventOnSpawnerCountChanged`
  (params (OldValue :type Integer) (NewValue :type Integer))
  ;[1 1 1] Setup level
  ;;[1 1 1] Bind to level clear event, enemy and spawner count changed events
  (`/Game/UI/Screens/WB_GameScreen.SetSpawnerCount` (`self.GameScreenWidget`) NewValue))

(event `EventOnEnemyCountChanged`
  (params (OldValue :type Integer) (NewValue :type Integer))
  ;[1 1 1] Setup level
  ;;[1 1 1] Bind to level clear event, enemy and spawner count changed events
  (`/Game/UI/Screens/WB_GameScreen.SetEnemyCount` (`self.GameScreenWidget`) NewValue))

(event `EventOnScoreChanged`
  (params (NewValue :type Integer) (OldValue :type Integer))
  ;[1 1 1] Setup level
  ;;[1 1 1] Bind to level clear event, enemy and spawner count changed events
  (`/Game/UI/Screens/WB_GameScreen.SetScore` (`self.GameScreenWidget`) (`KismetMathLibrary.Conv_IntToInt64` OldValue)))

(event `EventOnPlayerDefeatStarted`
  (params (Owner :type "Object Object Reference"))
  ;[1 1 1] Handle eplayer events
  (`/Game/UI/Screens/WB_GameScreen.ShowGameStateText` (`self.GameScreenWidget`) (`self.LevelClearedText`))
  (`KismetSystemLibrary.Delay` 5.0)
  (`/Game/UI/Screens/WB_GameScreen.HideGameStateText` (`self.GameScreenWidget`))
  (`GameplayStatics.OpenLevelBySoftObjectPtr` "/Game/LevelPrototyping/Maps/L_MainMenu.L_MainMenu"))

(event `EventOnPlayerSpawned`
  (params (OldPawn :type "Pawn Object Reference") (NewPawn :type "Pawn Object Reference"))
  (bind _returnvalue (`self.GetComponentByClass` NewPawn "/Script/TopDown2.CombatComponent"))
  ;[1 1 1] Handle eplayer events
  ;;[1 1 1] Binding to Player's health change and defeat events
  (`/Engine/EditorBlueprintResources/StandardMacros.IsValid` NewPawn
    (:`Is Valid`
      (`/Engine/EditorBlueprintResources/StandardMacros.IsValid` _returnvalue
        (:`Is Valid`
          (add `CombatComponent.OnHealthChanged` _returnvalue (`|CreateDelegate` :!event `EventOnPlayerHealthChanged`))
          (add `CombatComponent.OnDefeatStarted` _returnvalue (`|CreateDelegate` :!event `EventOnPlayerDefeatStarted`)))))))

(event `EventOnPlayerHealthChanged`
  (params (CombatComponent :type "CombatComponent Object Reference") (OldValue :type "Float (single-precision)") (NewValue :type "Float (single-precision)") (Initiator :type "Actor Object Reference"))
  ;[1 1 1] Handle eplayer events
  ;;[1 1 1] TODO: use viewmodels
  (`/Game/UI/WB_PlayerStatus.SetHealth` (`/Game/UI/Screens/WB_GameScreen.WB_PlayerStatus` (`self.GameScreenWidget`)) (`KismetMathLibrary.Conv_DoubleToInt64` (`CombatComponent.GetMaxHealth` CombatComponent)) (`KismetMathLibrary.Conv_DoubleToInt64` NewValue)))

(event `EventOnEnemyDefeatStarted`
  (params (Owner :type "Object Object Reference"))
  ;[1 1 1] Handle enemy events
  (`|ExecutionSequence`
    (:`then_0`
      (bind _returnvalue (`self.GetSpawnManager`))
      (`SpawnManager.ReturnEnemyToPool` _returnvalue Owner)
      (bind _asactor (cast `Actor` Owner))
      (`GameStateInterface.HandleEnemyDefeated` (`self.CurrentGameState`) _asactor))))

(event `OnEnemySpawned`
  (params (Enemy :type "Object Object Reference"))
  ;[1 1 1] Handle enemy events
  (bind _asactor (cast `Actor` Enemy))
  (`GameStateInterface.HandleEnemySpawned` (`self.CurrentGameState`) _asactor))

(event `EventLevelCleared`
  ;[1 1 1] Handle enemy events
  (`GameplayStatics.PlaySoundAtLocation` "/Game/Audio/Fantasy_Sound_Library/Mp3/Jingle_Achievement_00.Jingle_Achievement_00" (0.0 0.0 0.0) (struct) 1.0 1.0 0.0 null null null null)
  (`/Game/UI/Screens/WB_GameScreen.ShowGameStateText` (`self.GameScreenWidget`) (`self.LevelClearedText`))
  (`KismetSystemLibrary.Delay` 5.0)
  (`/Game/UI/Screens/WB_GameScreen.HideGameStateText` (`self.GameScreenWidget`))
  (`GameplayStatics.OpenLevelBySoftObjectPtr` "/Game/LevelPrototyping/Maps/L_MainMenu.L_MainMenu"))

(event `EventOnSpawnerDestroyed`
  (params (Owner :type "Object Object Reference"))
  (bind _asactor (cast `Actor` Owner))
  (`GameStateSpawnDestruction.HandleSpawnerDestroyed` (`self.CurrentGameState`) _asactor)
  (`self.K2_DestroyActor` _asactor))

(fn `DisplayGameStateText`
  (params (Time :type "Float (double-precision)") (Text :type Text)))

(fn `HideGameStateText`
  (`/Game/UI/Screens/WB_GameScreen.HideGameStateText` (`self.GameScreenWidget`))
  (return))

(fn `UserConstructionScript`)