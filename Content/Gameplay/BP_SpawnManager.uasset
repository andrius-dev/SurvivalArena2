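; Spawn manager that recycles defeated enemies through a pool and respawns them at spawners.
; On enemy defeat it calls ReturnEnemyToPool, waits on a Delay, then sends a random inactive pooled enemy to SpawnEnemy with a random CharacterSpawner.
; The pool and spawn functions are called here but defined elsewhere.
; BeginPlay only gathers BP_CharacterSpawner actors, as the logic binding their character-loaded debug print is disconnected.
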(event `self.ReceiveBeginPlay`
  (bind _outactors (`GameplayStatics.GetAllActorsOfClass` "/Game/Characters/AI/BP_CharacterSpawner.BP_CharacterSpawner_C")))

(event `OnCharacterLoaded_Event`
  (params (NewActor :type "Actor Object Reference") (Spawner :type "CharacterSpawner Object Reference"))
  (`KismetSystemLibrary.PrintString` (`KismetStringLibrary.BuildString_Vector` "" "" (`self.K2_GetActorLocation` Spawner))))

(event `OnEnemyDefeated_Event`
  (params (NewParam :type "Actor Object Reference"))
  (bind _returnvalue (`self.ReturnEnemyToPool` NewParam))
  (if _returnvalue
    _
    (else
      _))
  (`KismetSystemLibrary.LogString` (`KismetStringLibrary.BuildString_Name` "ReturnEnemyToPool failed, didn't find matching actor" "" (`KismetStringLibrary.Conv_StringToName` (`KismetSystemLibrary.GetDisplayName` NewParam))))
  (`KismetSystemLibrary.Delay` 5.0)
  (bind _returnvalue_2 (`self.GetRandomInactiveEnemyFromPool`))
  (`/Engine/EditorBlueprintResources/StandardMacros.IsValid` _returnvalue_2
    (:`Is Valid`
      (bind _outactors (`GameplayStatics.GetAllActorsOfClass` "/Script/TopDown2.CharacterSpawner"))
      (`self.SpawnEnemy` _returnvalue_2 (`KismetArrayLibrary.Array_Random` _outactors)))))

(fn `UserConstructionScript`)