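; Base enemy Blueprint that runs a basic behavior tree when possessed and can attack with a sword.
; Pawn sensing stores any seen Character as the target and writes it to the blackboard, as does a separate see-target event for an existing target.
; StartHitDetectionBP sphere-traces along the blade sockets against Pawn and WorldStatic objects, with debug drawing, and destroys the hit actor outright.
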(event `self.ReceivePossessed`
  (params (NewController :type "Controller Object Reference"))
  (`AIController.RunBehaviorTree` (`AIBlueprintHelperLibrary.GetAIController` self) "/Game/AI/BT_BasicEnemy.BT_BasicEnemy"))

(event `EventSeeTargetCharacter`
  (if (`KismetSystemLibrary.IsValid` (`self.TargetCharacter`))
    (`BlackboardComponent.SetValueAsObject` (`AIBlueprintHelperLibrary.GetBlackboard` null) (`self.KeyPlayerCharacter`) (stale `self.PawnSensing.OnSeePawn` _output_get) :!label _label)))

(event `self.PawnSensing.OnSeePawn`
  (params (Pawn :type "Pawn Object Reference"))
  (bind _ascharacter (cast `Character` Pawn)
    (:`then`
      (bind _output_get (set `self.TargetCharacter` _ascharacter))
      (goto _label))
    (:`CastFailed`
      (`KismetSystemLibrary.LogString` "AAA bleeee"))))

(fn `Start Hit Detection BP`
  (bind _sword (`self.Sword`))
  (bind (_outhit _returnvalue) (`KismetSystemLibrary.SphereTraceSingleForObjects` :`Start` (`SceneComponent.GetSocketLocation` _sword "BladeStart") :`End` (`SceneComponent.GetSocketLocation` _sword "BladeEnd") :`Radius` 20.0 :`ObjectTypes` (`|MakeArray` "ObjectTypeQuery3" "ObjectTypeQuery1" :!type "EObjectTypeQuery Enum") :`DrawDebugType` "ForDuration"))
  (if _returnvalue
    (`self.K2_DestroyActor` (`.HitActor` (`GameplayStatics.BreakHitResult` _outhit)))))

(fn `UserConstructionScript`)