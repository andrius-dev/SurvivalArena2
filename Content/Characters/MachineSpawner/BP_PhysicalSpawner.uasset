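; Destructible enemy spawner actor that periodically releases enemies into the level from a shared pool.
; On BeginPlay it finds the BP_SpawnManager and starts a looping timer, also spawning immediately.
; Each spawn takes a random inactive pooled enemy and has the manager place it at the arrow's location with the assembly box's rotation.
; On defeat it plays an explosion sound, reports to GameStateSpawnDestruction and destroys itself.
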(event `self.ReceiveBeginPlay`
  (`|ExecutionSequence`
    (:`then_0`
      (bind _returnvalue (`GameplayStatics.GetActorOfClass` "/Game/Gameplay/BP_SpawnManager.BP_SpawnManager_C"))
      (set `self.SpawnManager` _returnvalue)
      (`KismetSystemLibrary.K2_SetTimerDelegate` (delegate `SpawnEnemy`) (`self.EnemySpawnTime`) true false (`self.InitialSpawnDelay`))
      (`self.SpawnEnemy`))))

(event `SpawnEnemy`
  (bind _returnvalue (`SpawnManager.GetRandomInactiveEnemyFromPool` (`self.SpawnManager`)))
  (if (`KismetSystemLibrary.IsValidInterface` _returnvalue)
    (`SpawnManager.SpawnEnemyAtLocation` (`self.SpawnManager`) (`KismetSystemLibrary.Conv_InterfaceToObject` _returnvalue) (`SceneComponent.K2_GetComponentLocation` (`self.Arrow`)) (`SceneComponent.K2_GetComponentRotation` (`self.SM_AssemblyLineBox01`)))
    (else
      (`KismetSystemLibrary.PrintString` "Enemy is null"))))

(event `self.Combat.OnDefeat`
  (params (Owner :type "Object Object Reference"))
  (`GameplayStatics.PlaySoundAtLocation` "/Game/Audio/Explosion01.Explosion01" (`self.K2_GetActorLocation`) (struct) 1.0 1.0 0.0 null null null null)
  (bind _asgame_state_spawn_destruction (cast `GameStateSpawnDestruction` (`GameplayStatics.GetGameState`)))
  (`GameStateSpawnDestruction.HandleSpawnerDestroyed` _asgame_state_spawn_destruction self)
  (`self.K2_DestroyActor`))

(fn `UserConstructionScript`)