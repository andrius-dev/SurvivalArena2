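; Basic AI enemy for the survival game mode, which runs its behavior tree when possessed.
; Pawn sensing stores any seen Character, without a player check, as the blackboard's player target.
; The health component logs changes and, on death, reports the defeat to BP_GameModeSurvival.
; The hit detection function is empty, and its blade-socket sphere trace that destroys hit actors is disconnected.
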(event `self.ReceivePossessed`
  (params (NewController :type "Controller Object Reference"))
  (`AIController.RunBehaviorTree` (`AIBlueprintHelperLibrary.GetAIController` self) "/Game/Characters/AI/BT_BasicEnemy.BT_BasicEnemy"))

(event `self.PawnSensing.OnSeePawn`
  (params (Pawn :type "Pawn Object Reference"))
  ;[1 1 1] Setting player target in blackboard
  (bind _ascharacter (cast `Character` Pawn)
    (:`then`
      (bind _output_get (set `self.TargetCharacter` _ascharacter))
      (`BlackboardComponent.SetValueAsObject` (`AIBlueprintHelperLibrary.GetBlackboard` null) (`self.KeyPlayerCharacter`) _output_get))
    (:`CastFailed`
      (`KismetSystemLibrary.LogString` "AAA bleeee"))))

(event `self.HealthComponent.OnHealthChanged`
  (params (HealthComponent :type "HealthComponent Object Reference") (NewValue :type "Float (single-precision)") (OldValue :type "Float (single-precision)") (Initiator :type "Actor Object Reference"))
  ;[1 1 1] Health
  (`KismetSystemLibrary.LogString` (`KismetStringLibrary.BuildString_Double` "" "Got hit, current hp: " NewValue)))

(event `self.HealthComponent.OnDeath`
  (params (HealthComponent :type "HealthComponent Object Reference"))
  ;[1 1 1] Health
  (bind _asbp_game_mode_survival (cast `/Game/Gameplay/BP_GameModeSurvival` (`GameplayStatics.GetGameMode`)))
  (`/Game/Gameplay/BP_GameModeSurvival.OnEnemyDefeated_Event` _asbp_game_mode_survival HealthComponent self (`AIBlueprintHelperLibrary.GetAIController` self)))

(fn `Start Hit Detection BP`)

(fn `UserConstructionScript`)