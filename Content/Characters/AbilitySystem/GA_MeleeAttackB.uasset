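; GA_MeleeAttackB is a melee attack gameplay ability that commits, plays its montage and ends when the montage completes, blends out or is interrupted.
; Alongside the montage it starts waits for combo window start and end events, but only the end event is handled, removing all combo window loose tags from the avatar.
; Nodes that would swap previous and current combo window tags are disconnected and never run.
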(event `self.K2_ActivateAbility`
  (`self.K2_CommitAbility`)
  (`AbilityTask_PlayMontageAndWait.CreatePlayMontageAndWaitProxy` "None" (`self.Montage to Play`) 1.0 "None" false
    (:`then`
      (`AbilityTask_WaitGameplayEvent.WaitGameplayEvent` (struct :`TagName` "Event.ComboWindow.Start") null
        (:`then`
          (`AbilityTask_WaitGameplayEvent.WaitGameplayEvent` (struct :`TagName` "Event.ComboWindow.End") null
            (:`EventReceived`
              (`AbilitySystemBlueprintLibrary.RemoveLooseGameplayTags` (`self.GetAvatarActorFromActorInfo`) (`self.TagAllComboWindows`)))))))
    (:`OnCompleted`
      (`self.K2_EndAbility` :!label _label))
    (:`OnBlendOut`
      (goto _label))
    (:`OnInterrupted`
      (goto _label))))