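; GA_MeleeAttackA is a gameplay ability for a melee attack with a combo window.
; On activation it commits, plays its montage and waits for combo window start and end gameplay events.
; The start event adds a non-replicated loose combo window tag to the avatar; the end event removes it and ends the ability.
; Montage completion also ends the ability, without removing the tag.
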(event `self.K2_ActivateAbility`
  (`self.K2_CommitAbility`)
  (`AbilityTask_PlayMontageAndWait.CreatePlayMontageAndWaitProxy` "None" (`self.Montage to Play`)
    (:`then`
      (`AbilityTask_WaitGameplayEvent.WaitGameplayEvent` (struct :`TagName` "Event.ComboWindow.Start") null
        (:`then`
          (`AbilityTask_WaitGameplayEvent.WaitGameplayEvent` (struct :`TagName` "Event.ComboWindow.End") null
            (:`EventReceived`
              (`AbilitySystemBlueprintLibrary.RemoveLooseGameplayTags` (`self.GetAvatarActorFromActorInfo`) (`self.TagCurrentComboWindow`))
              (`self.K2_EndAbility`))))
        (:`EventReceived`
          (`AbilitySystemBlueprintLibrary.AddLooseGameplayTags` (`self.GetAvatarActorFromActorInfo`) (`self.TagCurrentComboWindow`)))))
    (:`OnCompleted`
      (`self.K2_EndAbility`))))