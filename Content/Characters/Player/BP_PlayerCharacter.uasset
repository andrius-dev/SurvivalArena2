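; Player character Blueprint that drives melee combat, dodging and jumping through the Gameplay Ability System.
; BeginPlay grants the abilities and initial attribute effect, and Enhanced Input actions activate abilities by gameplay tag.
; Melee hits detected by CombatComponent apply a damage effect to targets that have an ability system.
; A jump shadow decal appears while airborne, following a downward line trace to world Z zero until landing.
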(event OnHealthChanged(CombatComponent)
  (params (CombatComponent :type Combat%20Component%20Object%20Reference) (OldValue :type Float%20%28single-precision%29) (NewValue :type Float%20%28single-precision%29) (Initiator :type Actor%20Object%20Reference)))

(event OnDetectedMeleeHit(CombatComponent)
  (params (Owner :type Object%20Object%20Reference) (HitResults :type Array%20of%20Hit%20Result%20Structures))
  (for _array_element HitResults
    (Utilities|IsValid (Ability|GetAbilitySystemComponent (.HitActor (Collision|BreakHitResult _array_element)))
      (:Is%20Valid
        (GameplayEffects|ApplyGameplayEffectToTarget :self (Variables|Default|GetAbilitySystem) :GameplayEffectClass "/Game/Characters/AbilitySystem/GE_MeleeDamage.GE_MeleeDamage_C" :Target (Ability|GetAbilitySystemComponent (.HitActor (Collision|BreakHitResult _array_element))))))))

(event Input|EnhancedActionEvents|EnhancedInputActionIA_Attack_Melee
  (params (ActionValue :type Boolean) (ElapsedSeconds :type Float%20%28double-precision%29) (TriggeredSeconds :type Float%20%28double-precision%29) (InputAction :type Input%20Action%20Object%20Reference :default "/Game/Input/Actions/IA_Attack_Melee.IA_Attack_Melee"))
  ;[1 1 1] Input handling with abilities
  (Abilities|TryActivateAbilitiesbyTag (Variables|Default|GetAbilitySystem) (Variables|Default|GetTagsSwordAttack) true)
  (Abilities|TryActivateAbilitiesbyTag (Variables|Default|GetAbilitySystem) (Variables|Default|GetTagJumpAttack) true))

(event Input|EnhancedActionEvents|EnhancedInputActionIA_Dodge
  (params (ActionValue :type Boolean) (ElapsedSeconds :type Float%20%28double-precision%29) (TriggeredSeconds :type Float%20%28double-precision%29) (InputAction :type Input%20Action%20Object%20Reference :default "/Game/Input/Actions/IA_Dodge.IA_Dodge"))
  ;[1 1 1] Input handling with abilities
  (Abilities|TryActivateAbilitiesbyTag (Variables|Default|GetAbilitySystem) (Variables|Default|GetTagDodge) true))

(event Input|EnhancedActionEvents|EnhancedInputActionIA_Jump
  (params (ActionValue :type Boolean) (ElapsedSeconds :type Float%20%28double-precision%29) (TriggeredSeconds :type Float%20%28double-precision%29) (InputAction :type Input%20Action%20Object%20Reference :default "/Game/Input/Actions/IA_Jump.IA_Jump"))
  ;[1 1 1] Input handling with abilities
  (Abilities|TryActivateAbilitiesbyTag (Variables|Default|GetAbilitySystem) (Variables|Default|GetTagJump) true))

(event Input|EnhancedActionEvents|EnhancedInputActionIA_Movement
  (params (ActionValue :type Vector%202D%20Structure) (ElapsedSeconds :type Float%20%28double-precision%29) (TriggeredSeconds :type Float%20%28double-precision%29) (InputAction :type Input%20Action%20Object%20Reference :default "/Game/Input/Actions/IA_Movement.IA_Movement"))
  (:Started
    ;[1 1 1] Input handling with abilities
    (Abilities|TryActivateAbilitiesbyTag (Variables|Default|GetAbilitySystem) (Variables|Default|GetTagsMovement) true)))

(event EventBeginPlay
  (Utilities|FlowControl|Sequence
    (:then_0
      (bind _returnvalue (Rendering|Decal|SpawnDecalatLocation "/Game/Characters/M_JumpShadow.M_JumpShadow" "25.000000,50.000000,50.000000" (Transformation|GetActorLocation) "-90.000000,0.000000,0.000000" 0.0))
      (bind _output_get (Variables|Default|SetJumpDecal _returnvalue))
      (Development|SetHiddeninGame _output_get true false))
    (:then_1
      ;[1 1 1] Adding abilities
      (GameplayAbilities|GiveAbility (Variables|Default|GetAbilitySystem) "/Game/Characters/AbilitySystem/GA_MeleeAttackA.GA_MeleeAttackA_C" 0 -1)
      (GameplayAbilities|GiveAbility (Variables|Default|GetAbilitySystem) "/Game/Characters/AbilitySystem/GA_MeleeAttackB.GA_MeleeAttackB_C" 0 -1)
      (GameplayAbilities|GiveAbility (Variables|Default|GetAbilitySystem) "/Game/Characters/AbilitySystem/GA_Dodge.GA_Dodge_C" 0 -1)
      (GameplayAbilities|GiveAbility (Variables|Default|GetAbilitySystem) "/Game/Characters/AbilitySystem/GA_Jump.GA_Jump_C" 0 -1)
      (GameplayAbilities|GiveAbility (Variables|Default|GetAbilitySystem) "/Game/Characters/AbilitySystem/GA_MeleeJumpAttack.GA_MeleeJumpAttack_C" 0 -1)
      (GameplayEffects|ApplyGameplayEffectToSelf :self (Variables|Default|GetAbilitySystem) :GameplayEffectClass "/Game/Characters/AbilitySystem/GE_InitPlayerAttributes.GE_InitPlayerAttributes_C" :Level 1.0))))

(event EventOnJumped
  ;[0.8333 0.8333 0.8333] Jump shadow decal
  (Development|SetHiddeninGame (Variables|Default|GetJumpDecal) false false))

(event EventOnLanded
  (params (Hit :type Hit%20Result%20Structure%20%28by%20ref%29))
  ;[0.8333 0.8333 0.8333] Jump shadow decal
  (Development|SetHiddeninGame (Variables|Default|GetJumpDecal) true false))

(event EventTick
  (params (DeltaSeconds :type Float%20%28single-precision%29))
  ;[0.8333 0.8333 0.8333] Jump shadow decal
  (if (not (Variables|/Script/Engine.SceneComponent|GetbHiddenInGame (Variables|Default|GetJumpDecal)))
    (bind _impactpoint (CallFunction|GetGroundPosition))
    (Transformation|SetWorldLocation (Variables|Default|GetJumpDecal) _impactpoint false false)))

(event Input|KeyboardEvents|DebugKeyF
  (params (Key :type Key%20Structure :default "None") (ActionValue :type Input%20Action%20Value%20Structure))
  (:Pressed
    (Development|PrintString (Utilities|String|ToString(Float) (.ReturnValue (Class|AbilitySystemComponent|GetGameplayAttributeValue (Variables|Default|GetAbilitySystem) "(AttributeName=\"Health\",Attribute=/Script/TopDown2.CombatAttributeSet:Health,AttributeOwner=\"/Script/CoreUObject.Class'/Script/TopDown2.CombatAttributeSet'\")"))))))

(event Input|KeyboardEvents|1
  (params (Key :type Key%20Structure :default "None"))
  ;[1 1 1] Debug
  (:Pressed
    (Default|CallOnScoreAddPressed)))

(fn ConstructionScript)

(fn GetGroundPosition
  (bind _returnvalue (Transformation|GetActorLocation))
  (bind (_x _y) (Math|Vector|BreakVector _returnvalue))
  (bind _outhit (Collision|LineTraceByChannel _returnvalue (Math|Vector|MakeVector _x _y 0.0) "TraceTypeQuery1" false 0 "None"))
  (return (.ImpactPoint (Collision|BreakHitResult _outhit))))