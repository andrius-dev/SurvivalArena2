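; BP_DroneBullet is the projectile actor for the drone, damaging the player on contact.
; When its movement component activates, it sets velocity to the Arrow component's forward vector.
; On overlap with an actor implementing PlayerCharacterInterface, it applies fixed damage through that actor's combat component, crediting its owner, then destroys itself.
; A timer started at BeginPlay destroys bullets after TimeUntilDestruction.
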(event `self.ReceiveBeginPlay`
  (`KismetSystemLibrary.K2_SetTimerDelegate` (delegate `DestroySelf`) (`self.TimeUntilDestruction`)))

(event `DestroySelf`
  (`self.K2_DestroyActor`))

(event `self.ReceiveActorBeginOverlap`
  (params (OtherActor :type "Actor Object Reference"))
  (if (`KismetSystemLibrary.DoesImplementInterface` OtherActor "/Script/TopDown2.PlayerCharacterInterface")
    (bind _returnvalue (message `PlayerCharacterInterface.GetCombatComponent` OtherActor))
    (`CombatComponent.TakeDamage` _returnvalue 10.0 (`self.GetOwner`))
    (`self.K2_DestroyActor`)))

(event `self.ProjectileMovement.OnComponentActivated`
  (params (Component :type "ActorComponent Object Reference") (bReset :type Boolean))
  (bind _asprojectile_movement_component (cast `ProjectileMovementComponent` Component))
  (set `MovementComponent.Velocity` (`SceneComponent.GetForwardVector` (`self.Arrow`)) _asprojectile_movement_component))

(fn `UserConstructionScript`)