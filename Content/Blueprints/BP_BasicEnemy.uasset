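; Basic enemy pawn that chases pawns it spots through PawnSensing.
; On each sighting, IsKickableAss accepts player-controlled pawns or those passing a class comparison against BP_PickupItem, caching the result in IsSeeingAss.
; An accepted pawn is stored in AssToKick, and FollowAss issues an AI MoveTo toward the sensed pawn.
; There is no attack or lost-sight logic.
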(event `self.PawnSensing.OnSeePawn`
  (params (Pawn :type "Pawn Object Reference"))
  (bind _result (`self.IsKickableAss` Pawn))
  (if _result
    (set `self.AssToKick` Pawn)
    (`self.FollowAss`)))

(event `FollowAss`
  (if (`self.IsSeeingAss`)
    (`|AIMoveTo` self (0.0 0.0 0.0) (stale `self.PawnSensing.OnSeePawn` Pawn))))

(fn `IsKickableAss`
  (params (self2 :type "Pawn Object Reference"))
  (returns (Result :type Boolean))
  (bind _output_get (set `self.IsSeeingAss` (or (`GameplayStatics.ObjectIsA` "/Game/Blueprints/BP_PickupItem.BP_PickupItem" (`GameplayStatics.GetObjectClass` self2)) (`self.IsPlayerControlled` self2))))
  (return _output_get))

(fn `UserConstructionScript`)